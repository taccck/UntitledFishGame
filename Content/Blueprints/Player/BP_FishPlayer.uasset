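; BP_FishPlayer is the player Blueprint that animates casting and pulling out a fishing rod.
; A Fishing event, gated by a DoOnce until the animation finishes, checks the movement component's IsFishing flag to play either the cast or pull-out timeline.
; Each timeline drives the rod's relative pitch.
; Tick wakes the rod's rigid bodies every frame.
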(event EventFishing
  (Utilities|FlowControl|DoOnce false :!label _label
    (:Completed
      (if (Variables|/Script/UntitledFishGame.FishPlayerMovement|GetbIsFishing (Variables|Default|GetMoveComp))
        (bind _pullout (Timeline|StopFishing PlayFromStart)
          (:Update
            (Transformation|SetRelativeRotation (Variables|Default|GetFishingrod) (Math|Rotator|MakeRotator 0.0 _pullout 0.0) false false))
          (:Finished
            (goto _label Reset)))
        (else
          (bind _castrod (Timeline|StartFishing PlayFromStart)
            (:Update
              (Transformation|SetRelativeRotation (Variables|Default|GetFishingrod) (Math|Rotator|MakeRotator 0.0 _castrod 0.0) false false))
            (:Finished
              (goto _label Reset))))))))

(event EventTick
  (params (DeltaSeconds :type Float%20%28single-precision%29))
  (Class|PrimitiveComponent|WakeAllRigidBodies (Variables|Default|GetFishingrod)))

(fn ConstructionScript)